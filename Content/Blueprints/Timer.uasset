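; Level countdown timer actor with a box trigger that serves as the win point.
; Tick uses a one-second Delay to step Minutes and Seconds down, calling RestartGame on GM_Base when both reach zero.
; Any overlap with the box stops the timer, halts BP_Hero by zeroing walk speed and stopping jumps, then shows the Win widget and sets the QuitGame flag.
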(event OnComponentBeginOverlap(Box)
  (params (OverlappedComponent :type Primitive%20Component%20Object%20Reference) (OtherActor :type Actor%20Object%20Reference) (OtherComp :type Primitive%20Component%20Object%20Reference) (OtherBodyIndex :type Integer) (bFromSweep :type Boolean) (SweepResult :type Hit%20Result%20Structure%20%28by%20ref%29))
  (Variables|Default|SetStopTimer true)
  (bind _returnvalue (Actor|GetActorOfClass "/Game/Blueprints/Hero/BP_Hero.BP_Hero_C"))
  (Variables|Default|SetHeroRef _returnvalue)
  (Components|Movement|StopMovementImmediately (Variables|/Script/Engine.Character|GetCharacterMovement (Variables|Default|GetHeroRef)))
  (Variables|/Script/Engine.CharacterMovementComponent|SetMaxWalkSpeed (Variables|/Script/Engine.Character|GetCharacterMovement (Variables|Default|GetHeroRef)) 0.0)
  (Character|StopJumping (Variables|Default|GetHeroRef))
  (CallFunction|WinGame))

(event Custom|Win%20Game
  (bind _returnvalue (UserInterface|CreateWidget "/Game/Win.Win_C"))
  (UserInterface|Viewport|AddtoViewport _returnvalue 0)
  (Variables|Default|SetQuit%20game true))

(event EventTick
  (params (DeltaSeconds :type Float%20%28single-precision%29))
  (if (not (Variables|Default|GetStopTimer))
    (Utilities|FlowControl|Delay 1.0)
    (if (== (Variables|Default|GetSeconds) 0)
      (if (== (Variables|Default|GetMinutes) 0)
        (bind _asgm_base (Utilities|Casting|CastToGM_Base (Game|GetGameMode)))
        (Class|GameMode|RestartGame _asgm_base)
        (else
          (Variables|Default|SetSeconds 59)
          (Variables|Default|SetMinutes (- (Variables|Default|GetMinutes) 1))))
      (else
        (Variables|Default|SetSeconds (- (Variables|Default|GetSeconds) 1))))))

(fn ConstructionScript)