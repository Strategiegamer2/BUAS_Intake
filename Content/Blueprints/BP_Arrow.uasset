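; BP_Arrow is an arrow actor that travels along the spline owned by the BP_Hero actor.
; On BeginPlay it finds the hero, stores the reference and starts the MoveObject timeline, with play rate scaled by TimeToComplete to set the travel duration.
; Each update maps the timeline track to a distance along the spline and sets the arrow's world location and rotation to match.
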(event Custom|MoveArrow
  (bind _spineref (Variables|Default|GetSpineRef))
  (bind _spline (Variables|/Game/Blueprints/Hero/BP_Hero.BP_Hero_C|GetSpline _spineref))
  (Components|Timeline|SetPlayRate (Variables|Default|GetMoveObject) (/ 1.0 (Variables|Default|GetTimeToComplete)))
  (bind _movetrack (Timeline|MoveObject Play)
    (:Update
      (Transformation|SetActorTransform (Math|Transform|MakeTransform (Spline|GetLocationatDistanceAlongSpline _spline (Math|Float|Lerp 0.0 (Spline|GetSplineLength (Variables|/Game/Blueprints/Hero/BP_Hero.BP_Hero_C|GetSpline (Variables|Default|GetSpineRef))) _movetrack) "World") (Spline|GetRotationatDistanceAlongSpline _spline (Math|Float|Lerp 0.0 (Spline|GetSplineLength (Variables|/Game/Blueprints/Hero/BP_Hero.BP_Hero_C|GetSpline (Variables|Default|GetSpineRef))) _movetrack) "World") "1.000000,1.000000,1.000000")))))

(event EventBeginPlay
  (bind _returnvalue (Actor|GetActorOfClass "/Game/Blueprints/Hero/BP_Hero.BP_Hero_C"))
  (Variables|Default|SetSpineRef _returnvalue)
  (CallFunction|MoveArrow))

(fn ConstructionScript)